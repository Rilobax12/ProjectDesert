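; Tube light fixture Blueprint for the Derelict Workshop whose overall brightness is scaled by a single LuminanceFactor.
; The construction script multiplies the intensity of the main spot, base glow and reflection highlight lights by that factor.
; It also creates dynamic material instances to scale the godray opacity and the emissive color of the tube and cover meshes to match.
; The event graph holds no active logic.
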(event EventBeginPlay)

(event Collision|EventActorBeginOverlap
  (params (OtherActor :type Actor%20Object%20Reference)))

(event EventTick
  (params (DeltaSeconds :type Float%20%28single-precision%29)))

(fn ConstructionScript
  (bind _spotlight (Variables|Default|GetSpotLight))
  (bind _light (Variables|Default|Getlight))
  (bind _light_cover (Variables|Default|Getlight_cover))
  (bind _highlight (Variables|Default|Gethighlight))
  (bind _baselight (Variables|Default|GetBaselight))
  (bind _godrayfill (Variables|Default|GetGodrayfill))
  ;[1 1 1] Set intensity of main light
  (Rendering|Components|Light|SetIntensity _spotlight (* (Variables|/Script/Engine.LightComponentBase|GetIntensity _spotlight) (Variables|Light|GetLuminance%20Factor)))
  ;[1 1 1] Set intensity of the light makes the area around the tube appear to glow
  (Rendering|Components|Light|SetIntensity _baselight (* (Variables|/Script/Engine.LightComponentBase|GetIntensity _baselight) (Variables|Light|GetLuminance%20Factor)))
  ;[1 1 1] Set intensity of a light that provides extra highlights in reflections
  (Rendering|Components|Light|SetIntensity _highlight (* (Variables|/Script/Engine.LightComponentBase|GetIntensity _highlight) (Variables|Light|GetLuminance%20Factor)))
  ;[1 1 1] Create and set the godray intensity
  (bind _returnvalue (Rendering|Material|CreateDynamicMaterialInstance _godrayfill 0 "/Game/DerelictWorkshop/Materials/Instances/mi_godray_b.mi_godray_b" :!class /Script/Engine.PrimitiveComponent))
  (bind _returnvalue_2 (Rendering|Material|GetScalarParameterValue _returnvalue "Opacity" :!class /Script/Engine.MaterialInstanceDynamic))
  (Rendering|Material|SetScalarParameterValueonMaterials _godrayfill "Opacity" (* _returnvalue_2 (Variables|Light|GetLuminance%20Factor)))
  ;[1 1 1] Set the intensity of the emissive value on the light tube mesh
  (bind _returnvalue_3 (Rendering|Material|CreateDynamicMaterialInstance _light 0 "/Game/DerelictWorkshop/Materials/Instances/mi_light_b_emmissive.mi_light_b_emmissive" :!class /Script/Engine.PrimitiveComponent))
  (bind _returnvalue_4 (Rendering|Material|GetVectorParameterValue _returnvalue_3 "EmissiveMultiply" :!class /Script/Engine.MaterialInstanceDynamic))
  (Rendering|Material|SetVectorParameterValueonMaterials _light "EmissiveMultiply" (Math|Conversions|ToVector(LinearColor) (* _returnvalue_4 (Variables|Light|GetLuminance%20Factor))))
  ;[1 1 1] Set the intensity of the emissive value on the light tube cover mesh
  (bind _returnvalue_5 (Rendering|Material|CreateDynamicMaterialInstance _light_cover 0 "/Game/DerelictWorkshop/Materials/Instances/mi_light_b_translucent.mi_light_b_translucent" :!class /Script/Engine.PrimitiveComponent))
  (bind _returnvalue_6 (Rendering|Material|GetVectorParameterValue _returnvalue_5 "EmissiveMultiply" :!class /Script/Engine.MaterialInstanceDynamic))
  (Rendering|Material|SetVectorParameterValueonMaterials _light_cover "EmissiveMultiply" (Math|Conversions|ToVector(LinearColor) (* _returnvalue_6 (Variables|Light|GetLuminance%20Factor)))))