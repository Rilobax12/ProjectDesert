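; Switched-off variant of the light A fixture prop for the Derelict Workshop environment, with no runtime logic.
; The construction script creates dynamic material instances for the Light and LightCover meshes, from emissive and translucent materials respectively.
; It scales each EmissiveMultiply vector parameter by LuminanceFactor and writes it back, intended to keep the emissive at zero.
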(event EventBeginPlay)

(event Collision|EventActorBeginOverlap
  (params (OtherActor :type Actor%20Object%20Reference)))

(event EventTick
  (params (DeltaSeconds :type Float%20%28single-precision%29)))

(fn ConstructionScript
  (bind _light (Variables|Default|Getlight))
  (bind _light_cover (Variables|Default|Getlight_cover))
  ;[1 1 1] Make sure emissive values are at 0
  (bind _returnvalue (Rendering|Material|CreateDynamicMaterialInstance _light 0 "/Game/DerelictWorkshop/Materials/Instances/mi_light_a_emmissive.mi_light_a_emmissive" :!class /Script/Engine.PrimitiveComponent))
  (bind _returnvalue_2 (Rendering|Material|GetVectorParameterValue _returnvalue "EmissiveMultiply" :!class /Script/Engine.MaterialInstanceDynamic))
  (Rendering|Material|SetVectorParameterValueonMaterials _light "EmissiveMultiply" (Math|Conversions|ToVector(LinearColor) (* _returnvalue_2 (Variables|Light|GetLuminance%20Factor))))
  (bind _returnvalue_3 (Rendering|Material|CreateDynamicMaterialInstance _light_cover 0 "/Game/DerelictWorkshop/Materials/Instances/mi_light_a_translucent.mi_light_a_translucent" :!class /Script/Engine.PrimitiveComponent))
  (bind _returnvalue_4 (Rendering|Material|GetVectorParameterValue _returnvalue_3 "EmissiveMultiply" :!class /Script/Engine.MaterialInstanceDynamic))
  (Rendering|Material|SetVectorParameterValueonMaterials _light_cover "EmissiveMultiply" (Math|Conversions|ToVector(LinearColor) (* _returnvalue_4 (Variables|Light|GetLuminance%20Factor)))))