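; Swing line equipment that tethers the player to aimed-at surfaces for swinging.
; While Fire is held, a grid of line traces gathers hits each tick until one nearest an ideal point along the offset aim becomes the tether.
; Tethering spawns a left-hand cable and raises air control; each tick cancels velocity away from the anchor and ratchets down stored length.
; Jumping, landing or firing again releases it.
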(event EventBeginPlay
  (|CallParentFunction) ; This node is disabled and will not be called.\nDrag off pins to build functionality.
)

(event Collision|EventActorBeginOverlap
  (params (OtherActor :type Actor%20Object%20Reference))
  (|CallParentFunction OtherActor) ; This node is disabled and will not be called.\nDrag off pins to build functionality.
)

(event EventJump
  (CallFunction|UnTether))

(event EventStopJump)

(event EventInitialize
  (params (PlayerCharacter :type ALS%20Player%20Character%20BP%20Object%20Reference) (MovementComponent :type Character%20Movement%20Component%20Object%20Reference))
  (|CallParentFunction PlayerCharacter MovementComponent))

(event EventFire
  (Variables|Default|SetbTetherSearch true)
  (CallFunction|UnTether))

(event EventLanded
  (CallFunction|UnTether))

(event EventStopFire
  (Variables|Default|SetbTetherSearch false))

(event EventAimInput
  (params (AimVector :type Vector :default "0, 0, 0"))
  (Variables|Default|SetAimVector AimVector))

(event EventTick
  (params (DeltaSeconds :type Float%20%28single-precision%29))
  (Utilities|FlowControl|Sequence
    (:then_0
      (if (Variables|Default|GetbTetherSearch)
        (Utilities|Array|Clear (Variables|Default|GetTetherPoints))
        (Utilities|Array|Clear (Variables|Default|GetHitObjectArray))
        (CallFunction|TetherSearchFunction)
        (CallFunction|SortTethers)))
    (:then_1
      (if (Variables|Default|GetbTethered)
        (CallFunction|SwingForce)
        (CallFunction|ShortenTether)))))

(fn ConstructionScript
  (|CallParentFunction))

(fn TetherSearchFunction
  (bind _playercharacter (Variables|Default|GetPlayerCharacter))
  (bind _aimvector (Variables|Default|GetAimVector))
  (bind _returnvalue (Math|Conversions|RotationFromXVector _aimvector))
  (bind _returnvalue_2 (Transformation|GetActorLocation _playercharacter))
  (bind (_roll _pitch _yaw) (Math|Rotator|BreakRotator _returnvalue))
  (for _index (range 0 (- (* (Variables|Default|GetNumRays_X) (Variables|Default|GetNumRays_Y)) 1))
    (bind (_outhit _returnvalue_3) (Collision|LineTraceByChannel _returnvalue_2 (+ _returnvalue_2 (* (Math|Vector|GetForwardVector (Math|Rotator|MakeRotator 0.0 (+ (* (Math|Integer|%(Integer) _index (Variables|Default|GetNumRays_Y)) (Variables|Default|GetRaySpread_Y)) _pitch (* (Math|Conversions|ToFloat(Integer) (- (Variables|Default|GetNumRays_Y) 1)) (Variables|Default|GetRaySpread_Y) -0.5) (Variables|Default|GetTraceHeightOffset)) (+ (* (Math|Integer|%(Integer) (/ _index (Variables|Default|GetNumRays_Y)) (Variables|Default|GetNumRays_X)) (Variables|Default|GetRaySpread_X)) _yaw (* (Math|Conversions|ToFloat(Integer) (- (Variables|Default|GetNumRays_X) 1)) (Variables|Default|GetRaySpread_X) -0.5)))) (Variables|Default|GetRayLength))) "TraceTypeQuery1" false 0 "ForOneFrame"))
    (if _returnvalue_3
      (Utilities|Array|Add (Variables|Default|GetTetherPoints) (.Location (Collision|BreakHitResult _outhit)))
      (Utilities|Array|Add (Variables|Default|GetHitObjectArray) (.HitActor (Collision|BreakHitResult _outhit)))))
  (return))

(fn SortTethers
  (if (> (Utilities|Array|Length (Variables|Default|GetTetherPoints)) 0)
    (CallFunction|SetIdealTether)
    (Variables|Default|SetClosestIdeal 1e+06)
    (Variables|Default|SetTetherIndex -1)
    (for (_array_element _array_index) (Variables|Default|GetTetherPoints)
      (if (< (Math|Vector|VectorLength (- _array_element (Variables|Default|GetIdealTether))) (Variables|Default|GetClosestIdeal))
        (Variables|Default|SetTetherPoint _array_element)
        (Variables|Default|SetClosestIdeal (Math|Vector|VectorLength (- _array_element (Variables|Default|GetIdealTether))))
        (Variables|Default|SetTetherIndex _array_index)))
    (Variables|Default|SetTetherLength (Math|Vector|VectorLength (- (Variables|Default|GetTetherPoint) (Transformation|GetActorLocation (Variables|Default|GetPlayerCharacter)))))
    (CallFunction|Tether)
    (return)
    (else
      (return))))

(fn SetIdealTether
  (bind _aimvector (Variables|Default|GetAimVector))
  (bind _returnvalue (Math|Conversions|RotationFromXVector _aimvector))
  (Variables|Default|SetIdealTether (+ (Transformation|GetActorLocation (Variables|Default|GetPlayerCharacter)) (* (Math|Vector|GetForwardVector (Math|Rotator|MakeRotator 0.0 (+ (.pitch _returnvalue) (Variables|Default|GetTraceHeightOffset)) (.yaw _returnvalue))) 5e+02)))
  (return))

(fn SwingForce
  (bind _tetherpoint (Variables|Default|GetTetherPoint))
  (bind _playercharacter (Variables|Default|GetPlayerCharacter))
  (bind _returnvalue (Transformation|GetVelocity _playercharacter))
  (bind _returnvalue_2 (Transformation|GetActorLocation _playercharacter))
  (bind _returnvalue_3 (- _returnvalue_2 _tetherpoint))
  (bind _returnvalue_4 (Math|Vector|Normalize _returnvalue_3))
  (if (> (Math|Vector|DotProduct (Math|Vector|Normalize _returnvalue) _returnvalue_4) 0.0)
    (Variables|/Script/Engine.MovementComponent|SetVelocity (Variables|Default|GetPlayerMovementComponent) (- _returnvalue (* (Math|Vector|ProjectVectorontoVector _returnvalue _returnvalue_4) 1.0)))))

(fn ShortenTether
  (bind _tetherpoint (Variables|Default|GetTetherPoint))
  (bind _playercharacter (Variables|Default|GetPlayerCharacter))
  (bind _returnvalue (Transformation|GetActorLocation _playercharacter))
  (bind _returnvalue_2 (- _returnvalue _tetherpoint))
  (bind _returnvalue_3 (Math|Vector|VectorLength _returnvalue_2))
  (if (< _returnvalue_3 (Variables|Default|GetTetherLength))
    (Variables|Default|SetTetherLength _returnvalue_3)))

(fn Tether
  (bind _hitobjectarray (Variables|Default|GetHitObjectArray))
  (bind _tetherindex (Variables|Default|GetTetherIndex))
  (bind _playercharacter (Variables|Default|GetPlayerCharacter))
  (bind _output (Utilities|Array|Get(acopy) _hitobjectarray _tetherindex))
  (Variables|Default|SetbTetherSearch false)
  (Variables|Default|SetbTethered true)
  (Variables|/Script/Engine.CharacterMovementComponent|SetAirControl (Variables|Default|GetPlayerMovementComponent) 2.0)
  (Variables|/Game/AdvancedLocomotionV2/Blueprints/ALS_Player_CharacterBP.ALS_Player_CharacterBP_C|SetTethered _playercharacter true)
  (bind _returnvalue (Game|SpawnActorfromClass "/Game/Aidan_WIP/BP_CableActor.BP_CableActor_C" (Transformation|GetActorTransform _playercharacter) "Undefined" _playercharacter 0))
  (bind _output_get (Variables|Default|SetCable _returnvalue))
  (Transformation|AttachComponentToComponent _output_get (Variables|/Script/Engine.Character|GetMesh _playercharacter) "hand_l" "SnapToTarget" "SnapToTarget" "SnapToTarget" true)
  (Class|CableComponent|SetAttachEndto (Variables|/Game/Aidan_WIP/BP_CableActor.BP_CableActor_C|GetCable (Variables|Default|GetCable)) _output "" "")
  (Variables|/Script/CableComponent.CableComponent|SetEndLocation (Variables|/Game/Aidan_WIP/BP_CableActor.BP_CableActor_C|GetCable (Variables|Default|GetCable)) (Math|Transform|InverseTransformLocation (Transformation|GetActorTransform _output) (Variables|Default|GetTetherPoint))))

(fn UnTether
  (bind _cable (Variables|Default|GetCable))
  (Variables|Default|SetbTethered false)
  (Variables|/Game/AdvancedLocomotionV2/Blueprints/ALS_Player_CharacterBP.ALS_Player_CharacterBP_C|SetTethered (Variables|Default|GetPlayerCharacter) false)
  (Utilities|IsValid _cable
    (:Is%20Valid
      (Actor|DestroyActor _cable)
      (Variables|/Script/Engine.CharacterMovementComponent|SetAirControl (Variables|Default|GetPlayerMovementComponent) 0.05))))