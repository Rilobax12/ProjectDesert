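; Jetpack equipment that thrusts the player character while jump is held, draining a limited energy pool.
; Jump toggles a Tick gate that spends energy and calls JetpackForce, which tapers steering near max horizontal speed and scales lift by vertical velocity.
; Shutoff starts recharge after a retriggerable delay, and thrust re-engages once enough energy returns if jump is held while falling.
; Tick also prints the energy ratio on screen.
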(event Custom|JetpackRechargeEvent
  (Utilities|FlowControl|RetriggerableDelay (Variables|Default|GetJetpack_RechargeDelay))
  (Variables|Default|SetbJetpack_canRecharge true))

(event Custom|JetpackOn
  (Variables|Default|SetbJetpackOn true)
  (Utilities|FlowControl|Gate true) ; enters at Open
)

(event Custom|JetpackOff
  (CallFunction|JetpackRechargeEvent)
  (Variables|Default|SetbJetpackOn false)
  (Utilities|FlowControl|Gate true) ; enters at Close
)

(event EventBeginPlay
  (|CallParentFunction) ; This node is disabled and will not be called.\nDrag off pins to build functionality.
)

(event Collision|EventActorBeginOverlap
  (params (OtherActor :type Actor%20Object%20Reference))
  (|CallParentFunction OtherActor) ; This node is disabled and will not be called.\nDrag off pins to build functionality.
)

(event EventJump
  (Variables|Default|SetbJumpHeld true)
  (CallFunction|Jetpackon))

(event EventStopJump
  (Variables|Default|SetbJumpHeld false)
  (CallFunction|JetpackOff))

(event EventInitialize
  (params (PlayerCharacter :type ALS%20Player%20Character%20BP%20Object%20Reference) (MovementComponent :type Character%20Movement%20Component%20Object%20Reference))
  (|CallParentFunction PlayerCharacter MovementComponent)
  (Variables|Default|SetJetpack_energyCurrent (Variables|Default|GetJetpack_energyMax)))

(event EventTick
  (params (DeltaSeconds :type Float%20%28single-precision%29))
  (Utilities|FlowControl|Sequence
    (:then_0
      (CallFunction|JetpackRechargeTick)
      (Development|PrintString (Utilities|String|ToString(Float) (/ (Variables|Default|GetJetpack_energyCurrent) (Variables|Default|GetJetpack_energyMax))) true true "(R=0.000000,G=0.660000,B=1.000000,A=1.000000)" (Utilities|Time|GetWorldDeltaSeconds)))
    (:then_1
      (Utilities|FlowControl|Gate true
        (:Exit
          (Variables|Default|SetbJetpack_canRecharge false)
          (Variables|Default|SetJetpack_energyCurrent (Math|Float|Clamp(Float) (- (Variables|Default|GetJetpack_energyCurrent) (* (Variables|Default|GetJetpack_energyUseRate) (Utilities|Time|GetWorldDeltaSeconds))) 0.0 (Variables|Default|GetJetpack_energyMax)))
          (if (> (Variables|Default|GetJetpack_energyCurrent) 0.0)
            (CallFunction|JetpackForce)
            (else
              (CallFunction|JetpackOff))))))))

(fn ConstructionScript
  (|CallParentFunction))

(fn JetpackForce
  (bind _playercharacter (Variables|Default|GetPlayerCharacter))
  (bind _playercharacter_2 (Variables|Default|GetPlayerCharacter))
  (bind _playercharacter_3 (Variables|Default|GetPlayerCharacter))
  (bind _moveforward (Variables|Default|GetMoveForward))
  (bind _moveright (Variables|Default|GetMoveRight))
  (bind _moveforward_2 (Variables|Default|GetMoveForward))
  (bind _moveright_2 (Variables|Default|GetMoveRight))
  (bind _jetpack_horizontal_bias (Variables|Default|GetJetpack_Horizontal_Bias))
  (bind _jetpackmaxhorizontalvelocity (Variables|Default|GetJetpackMaxHorizontalVelocity))
  (bind _returnvalue (Transformation|GetVelocity _playercharacter_2))
  (bind _returnvalue_2 (Transformation|GetVelocity _playercharacter))
  (bind _returnvalue_3 (Transformation|GetActorTransform _playercharacter_3))
  (bind _returnvalue_4 (Transformation|GetActorTransform _playercharacter_2))
  (bind _returnvalue_5 (Math|Vector|MakeVector _moveforward_2 _moveright_2 0.0))
  (bind _z (Math|Vector|BreakVector _returnvalue_2))
  (bind _returnvalue_6 (Math|Vector|Normalize _returnvalue_5))
  (bind _returnvalue_7 (Math|Transform|InverseTransformDirection _returnvalue_4 _returnvalue))
  (bind (_x _y) (Math|Vector|BreakVector _returnvalue_7))
  (bind _returnvalue_8 (Math|Vector|MakeVector 0.0 0.0 _z))
  (bind _returnvalue_9 (Math|Vector|Normalize _returnvalue_8))
  (bind _returnvalue_10 (Math|Vector|VectorLength _returnvalue_8))
  (bind _returnvalue_11 (Math|Vector|MakeVector _x _y 0.0))
  (bind _returnvalue_12 (Math|Float|Absolute(Float) _y))
  (bind _returnvalue_13 (Math|Float|Absolute(Float) _x))
  (bind _returnvalue_14 (Math|Vector|DotProduct _returnvalue_9 "0, 0,1.000000"))
  (bind _returnvalue_15 (Math|Vector|Normalize _returnvalue_11))
  (bind _returnvalue_16 (Math|Vector|DotProduct _returnvalue_6 _returnvalue_15))
  (bind _returnvalue_17 (* _returnvalue_10 _returnvalue_14))
  (bind _returnvalue_18 (* _returnvalue_16 _returnvalue_12))
  (bind _returnvalue_19 (* _returnvalue_16 _returnvalue_13))
  (bind _returnvalue_20 (Math|Float|MapRangeClamped _returnvalue_18 0.0 _jetpackmaxhorizontalvelocity 1.0 0.0))
  (bind _returnvalue_21 (Math|Float|MapRangeClamped _returnvalue_19 0.0 _jetpackmaxhorizontalvelocity 1.0 0.0))
  (bind _returnvalue_22 (* _moveforward _jetpack_horizontal_bias _returnvalue_21))
  (bind _returnvalue_23 (* _moveright _jetpack_horizontal_bias _returnvalue_20))
  (bind _returnvalue_24 (Math|Vector|MakeVector _returnvalue_22 _returnvalue_23 1.0))
  (bind _returnvalue_25 (Math|Vector|Normalize _returnvalue_24))
  (bind _returnvalue_26 (Math|Transform|TransformDirection _returnvalue_3 _returnvalue_25))
  (bind (_x_2 _y_2 _z_2) (Math|Vector|BreakVector _returnvalue_26))
  (Physics|AddForce (Variables|Default|GetPlayerMovementComponent) (* (Math|Vector|MakeVector _x_2 _y_2 (* _z_2 (* (Math|Float|MapRangeClamped _returnvalue_17 -1e+03 0.0 2.0 1.0) (Math|Float|MapRangeClamped _returnvalue_17 0.0 3e+03 1.0 0.0)))) (* (Variables|Default|GetJetpack_force) (Variables|/Script/Engine.CharacterMovementComponent|GetMass (Variables|Default|GetPlayerMovementComponent)) 9.8))))

(fn JetpackRechargeTick
  (if (Math|Boolean|ANDBoolean (Variables|Default|GetbJetpack_canRecharge) (not (Variables|Default|GetbJetpackOn)) (!= (Variables|Default|GetJetpack_energyCurrent) (Variables|Default|GetJetpack_energyMax)))
    (Variables|Default|SetJetpack_energyCurrent (Math|Float|Clamp(Float) (+ (Variables|Default|GetJetpack_energyCurrent) (* (Variables|Default|GetJetpack_energyRechargeRate) (Utilities|Time|GetWorldDeltaSeconds))) 0.0 (Variables|Default|GetJetpack_energyMax)))
    (if (Math|Boolean|ANDBoolean (>= (Variables|Default|GetJetpack_energyCurrent) 15.0) (Variables|Default|GetbJumpHeld) (AI|Components|NavMovement|IsFalling (Variables|Default|GetPlayerMovementComponent)))
      (CallFunction|JetPackon))))