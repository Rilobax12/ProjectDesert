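; Swing-line equipment that tethers the player to a surface so they can swing, releasing on jump or landing.
; While fire is held and no tether is found, each tick casts a debug-drawn grid of line traces around the aim vector and attaches to the hit nearest an ideal point along that aim.
; While tethered, a force opposes velocity away from the anchor, and the recorded tether length only shrinks.
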(event EventBeginPlay
  (|CallParentFunction) ; This node is disabled and will not be called.\nDrag off pins to build functionality.
)

(event Collision|EventActorBeginOverlap
  (params (OtherActor :type Actor%20Object%20Reference))
  (|CallParentFunction OtherActor) ; This node is disabled and will not be called.\nDrag off pins to build functionality.
)

(event EventJump
  (CallFunction|UnTether))

(event EventStopJump)

(event EventInitialize
  (params (PlayerCharacter :type ALS%20Player%20Character%20BP%20Object%20Reference) (MovementComponent :type Character%20Movement%20Component%20Object%20Reference))
  (|CallParentFunction PlayerCharacter MovementComponent))

(event EventFire
  (Variables|Default|SetbTetherSearch true))

(event EventLanded
  (CallFunction|UnTether))

(event EventStopFire
  (Variables|Default|SetbTetherSearch false))

(event EventAimInput
  (params (AimVector :type Vector :default "0, 0, 0"))
  (Variables|Default|SetAimVector AimVector))

(event EventTick
  (params (DeltaSeconds :type Float%20%28single-precision%29))
  (Utilities|FlowControl|Sequence
    (:then_0
      (if (Variables|Default|GetbTetherSearch)
        (Utilities|Array|Clear (Variables|Default|GetTetherPoints))
        (CallFunction|TetherSearchFunction)
        (CallFunction|SortTethers)))
    (:then_1
      (if (Variables|Default|GetbTethered)
        (CallFunction|SwingForce)
        (CallFunction|ShortenTether)))))

(fn ConstructionScript
  (|CallParentFunction))

(fn TetherSearchFunction
  (bind _playercharacter (Variables|Default|GetPlayerCharacter))
  (bind _aimvector (Variables|Default|GetAimVector))
  (bind _returnvalue (Math|Conversions|RotationFromXVector _aimvector))
  (bind _returnvalue_2 (Transformation|GetActorLocation _playercharacter))
  (bind (_roll _pitch _yaw) (Math|Rotator|BreakRotator _returnvalue))
  (for _index (range 0 (- (* (Variables|Default|GetNumRays_X) (Variables|Default|GetNumRays_Y)) 1))
    (bind (_outhit _returnvalue_3) (Collision|LineTraceByChannel _returnvalue_2 (+ _returnvalue_2 (* (Math|Vector|GetForwardVector (Math|Rotator|MakeRotator 0.0 (+ (* (Math|Integer|%(Integer) _index (Variables|Default|GetNumRays_Y)) (Variables|Default|GetRaySpread_Y)) _pitch (* (Math|Conversions|ToFloat(Integer) (- (Variables|Default|GetNumRays_Y) 1)) (Variables|Default|GetRaySpread_Y) -0.5) (Variables|Default|GetTraceHeightOffset)) (+ (* (Math|Integer|%(Integer) (/ _index (Variables|Default|GetNumRays_Y)) (Variables|Default|GetNumRays_X)) (Variables|Default|GetRaySpread_X)) _yaw (* (Math|Conversions|ToFloat(Integer) (- (Variables|Default|GetNumRays_X) 1)) (Variables|Default|GetRaySpread_X) -0.5)))) (Variables|Default|GetRayLength))) "TraceTypeQuery1" false 0 "ForOneFrame"))
    (if _returnvalue_3
      (Utilities|Array|Add (Variables|Default|GetTetherPoints) (.Location (Collision|BreakHitResult _outhit)))))
  (return))

(fn SortTethers
  (if (> (Utilities|Array|Length (Variables|Default|GetTetherPoints)) 0)
    (CallFunction|SetIdealTether)
    (Variables|Default|SetClosestIdeal 1e+06)
    (for _array_element (Variables|Default|GetTetherPoints)
      (if (< (Math|Vector|VectorLength (- _array_element (Variables|Default|GetIdealTether))) (Variables|Default|GetClosestIdeal))
        (Variables|Default|SetTetherPoint _array_element)
        (Variables|Default|SetClosestIdeal (Math|Vector|VectorLength (- _array_element (Variables|Default|GetIdealTether))))))
    (Variables|Default|SetTetherLength (Math|Vector|VectorLength (- (Variables|Default|GetTetherPoint) (Transformation|GetActorLocation (Variables|Default|GetPlayerCharacter)))))
    (CallFunction|Tether)
    (return)
    (else
      (return))))

(fn SetIdealTether
  (Variables|Default|SetIdealTether (+ (Transformation|GetActorLocation (Variables|Default|GetPlayerCharacter)) (* (Variables|Default|GetAimVector) 1e+03)))
  (return))

(fn SwingForce
  (bind _playercharacter (Variables|Default|GetPlayerCharacter))
  (bind _tetherpoint (Variables|Default|GetTetherPoint))
  (bind _returnvalue (Transformation|GetActorLocation _playercharacter))
  (bind _returnvalue_2 (Transformation|GetVelocity _playercharacter))
  (bind _returnvalue_3 (- _returnvalue _tetherpoint))
  (bind _returnvalue_4 (Math|Vector|ProjectVectorontoVector _returnvalue_2 _returnvalue_3))
  (if (> (Math|Vector|DotProduct _returnvalue_4 _returnvalue_3) 0.0)
    (Physics|AddForce (Variables|Default|GetPlayerMovementComponent) (* _returnvalue_4 -1e+04))))

(fn ShortenTether
  (bind _tetherpoint (Variables|Default|GetTetherPoint))
  (bind _playercharacter (Variables|Default|GetPlayerCharacter))
  (bind _returnvalue (Transformation|GetActorLocation _playercharacter))
  (bind _returnvalue_2 (- _returnvalue _tetherpoint))
  (bind _returnvalue_3 (Math|Vector|VectorLength _returnvalue_2))
  (if (< _returnvalue_3 (Variables|Default|GetTetherLength))
    (Variables|Default|SetTetherLength _returnvalue_3)))

(fn Tether
  (Variables|Default|SetbTetherSearch false)
  (Variables|Default|SetbTethered true)
  (Variables|/Game/AdvancedLocomotionV2/Blueprints/ALS_Player_CharacterBP.ALS_Player_CharacterBP_C|SetTethered (Variables|Default|GetPlayerCharacter) true))

(fn UnTether
  (Variables|Default|SetbTethered false)
  (Variables|/Game/AdvancedLocomotionV2/Blueprints/ALS_Player_CharacterBP.ALS_Player_CharacterBP_C|SetTethered (Variables|Default|GetPlayerCharacter) false))