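; Player-controlled trike vehicle pawn that maps player input to driving and camera look.
; On BeginPlay it calls InitializeAllSystems; the driving logic behind that and the other vehicle calls is not defined in these graphs.
; Move axes feed clamped engine throttle and steering, and the Jump action holds the handbrake while pressed.
; Turn and LookUp axes drive controller yaw and pitch.
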(event EventBeginPlay
  (Class|VehiclePhysicsActor|InitializeAllSystems))

(event Input|ActionEvents|InputActionJump
  (params (Key :type Key%20Structure))
  (:Pressed
    (Class|VehiclePhysicsActor|SetHandbrake true))
  (:Released
    (Class|VehiclePhysicsActor|SetHandbrake false)))

(event Input|AxisEvents|InputAxisMoveForward
  (params (AxisValue :type Float%20%28single-precision%29))
  (Class|VehiclePhysicsActor|SetEngineThrottle (Math|Float|Clamp(Float) AxisValue -1.0)))

(event Input|AxisEvents|InputAxisMoveRight
  (params (AxisValue :type Float%20%28single-precision%29))
  (Class|VehiclePhysicsActor|SetSteering AxisValue))

(event Input|AxisEvents|InputAxisLookUp
  (params (AxisValue :type Float%20%28single-precision%29))
  (Pawn|Input|AddControllerPitchInput AxisValue))

(event Input|AxisEvents|InputAxisTurn
  (params (AxisValue :type Float%20%28single-precision%29))
  (Pawn|Input|AddControllerYawInput AxisValue))

(fn ConstructionScript)