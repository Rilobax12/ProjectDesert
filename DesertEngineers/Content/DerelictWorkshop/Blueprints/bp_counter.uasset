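; A workshop counter prop Blueprint with five door components that can be configured per instance.
; The Construction Script gathers the doors into an array and uses matching DoorsVisible and DoorRotation arrays to set each door's visibility and relative yaw.
; Shadow casting follows visibility, so hidden doors cast no shadow.
; The EventGraph holds only disabled default events, so the Blueprint adds no runtime logic.
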(event EventBeginPlay)

(event Collision|EventActorBeginOverlap
  (params (OtherActor :type Actor%20Object%20Reference)))

(event EventTick
  (params (DeltaSeconds :type Float%20%28single-precision%29)))

(fn ConstructionScript
  (bind _output_get (Variables|DoorParameters|SetDoors (Utilities|Array|MakeArray (Variables|Default|Getdoor_1) (Variables|Default|Getdoor_2) (Variables|Default|Getdoor_3) (Variables|Default|Getdoor_4) (Variables|Default|Getdoor_5))))
  ;[1 1 1] For each door determine visibility and rotation
  (for (_array_element _array_index) _output_get
    ;[1 1 1] Set the door's visibility and ensure that shadow casting is consistent with visibility
    (Rendering|SetVisibility _array_element (Utilities|Array|Get(acopy) (Variables|DoorParameters|GetDoors%20Visible?) _array_index) false)
    (Rendering|SetCastShadow _array_element (Utilities|Array|Get(acopy) (Variables|DoorParameters|GetDoors%20Visible?) _array_index))
    ;[1 1 1] Set the door's rotation
    (Transformation|SetRelativeRotation _array_element (Math|Rotator|MakeRotator 0.0 0.0 (Utilities|Array|Get(acopy) (Variables|DoorParameters|GetDoor%20Rotation) _array_index)) false false)))