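; Outside-curtain Blueprint whose construction script draws a configurable sun shape on its curtain through a dynamic material instance.
; An assigned directional light supplies the sun's direction and color, and its pitch updates SunHeight.
; Without one, SunHeight and actor yaw set the direction, and height blends the color from orange to pale yellow.
; Brightness, radius and hardness are always applied, and the RefreshMaterial checkbox acts as a self-resetting rerun trigger.
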(fn ConstructionScript
  (bind _returnvalue (Rendering|Material|CreateDynamicMaterialInstance (Variables|Default|Getoutside_curtain_b) 0 "/Game/DerelictWorkshop/Materials/Instances/mi_outside_curtains.mi_outside_curtains" :!class /Script/Engine.PrimitiveComponent)) ; Set up material to change based on sun direction
  (Variables|Default|SetSky%20material _returnvalue)
  (if (Variables|Default|GetRefresh%20material) ; Updating bool in details panel causes construction script to run again
    _
    (else
      _))
  (Variables|Default|SetRefresh%20material false)
  (Utilities|IsValid (Variables|Default|GetDirectional%20light%20actor) ; Has a directional light been assigned?
    (:Is%20Valid
      ;[1 1 1] Set the sun shape's location and color based on the selected light actor
      (Rendering|Material|SetVectorParameterValue (Variables|Default|GetSky%20material) "Light direction" (Math|Conversions|ToLinearColor(Vector) (Math|Rotator|GetRotationXVector (Transformation|GetActorRotation (Variables|Default|GetDirectional%20light%20actor)))) :!class /Script/Engine.MaterialInstanceDynamic)
      (Rendering|Material|SetVectorParameterValue (Variables|Default|GetSky%20material) "Sun color" (Math|Conversions|ToLinearColor(Color) (Variables|/Script/Engine.LightComponentBase|GetLightColor (Variables|/Script/Engine.Light|GetLightComponent (Variables|Default|GetDirectional%20light%20actor)))) :!class /Script/Engine.MaterialInstanceDynamic)
      (Variables|Overridesettings|SetSun%20height (Math|Float|MapRangeUnclamped (.Pitch (Math|Rotator|BreakRotator (Transformation|GetActorRotation (Variables|Default|GetDirectional%20light%20actor)))) 0.0 -9e+01 0.0 1.0)))
    (:Is%20Not%20Valid
      ;[1 1 1] Set the sun shape's location and color based on custom value
      (Rendering|Material|SetVectorParameterValue (Variables|Default|GetSky%20material) "Light direction" (Math|Conversions|ToLinearColor(Vector) (Math|Rotator|GetRotationXVector (Math|Rotator|MakeRotator 0.0 (Math|Float|MapRangeUnclamped (Variables|Overridesettings|GetSun%20height) -1.0 1.0 9e+01 -9e+01) (.Yaw (Math|Rotator|BreakRotator (Transformation|GetActorRotation)))))) :!class /Script/Engine.MaterialInstanceDynamic)
      (Rendering|Material|SetVectorParameterValue (Variables|Default|GetSky%20material) "Sun color" (Math|Color|Lerp(LinearColor) "(R=1.000000,G=0.221000,B=0.040000,A=1.000000)" "(R=0.954000,G=0.901000,B=0.744120,A=1.000000)" (Math|Float|Clamp(Float) (+ (Variables|Overridesettings|GetSun%20height) 0.2))) :!class /Script/Engine.MaterialInstanceDynamic)))
  ;[1 1 1] Set the sun shape's appearance
  (Rendering|Material|SetScalarParameterValue (Variables|Default|GetSky%20material) "Sun brightness" (Variables|Default|GetSun%20brightness) :!class /Script/Engine.MaterialInstanceDynamic)
  (Rendering|Material|SetScalarParameterValue (Variables|Default|GetSky%20material) "Sun Radius" (Variables|Default|GetSun%20Radius) :!class /Script/Engine.MaterialInstanceDynamic)
  (Rendering|Material|SetScalarParameterValue (Variables|Default|GetSky%20material) "Sun Hardness" (Variables|Default|GetSun%20Hardness) :!class /Script/Engine.MaterialInstanceDynamic))