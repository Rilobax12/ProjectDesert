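; Control panel prop for the Derelict Workshop with a switch button and screen that appear on or off according to a SwitchPositionOn flag.
; The construction script creates dynamic material instances for the button and screen, rotates the switch, and keeps their EmissiveMultiply glow when on or zeroes it when off.
; The state is applied only at construction, as the event graph holds no runtime logic.
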(event EventBeginPlay)

(event Collision|EventActorBeginOverlap
  (params (OtherActor :type Actor%20Object%20Reference)))

(event EventTick
  (params (DeltaSeconds :type Float%20%28single-precision%29)))

(fn ConstructionScript
  (bind _switch_button (Variables|Default|Getswitch_button))
  (bind _staticmeshcomponent (Variables|Debug|GetStaticMeshComponent))
  ;[1 1 1] Set up materials to change based on switch position
  (bind _returnvalue (Rendering|Material|CreateDynamicMaterialInstance _switch_button 0 "/Game/DerelictWorkshop/Materials/Instances/mi_electrical_glow.mi_electrical_glow" :!class /Script/Engine.PrimitiveComponent))
  (bind _returnvalue_2 (Rendering|Material|CreateDynamicMaterialInstance (Variables|Debug|GetStaticMeshComponent) 1 "/Game/DerelictWorkshop/Materials/Instances/mi_control_panel_screen.mi_control_panel_screen" :!class /Script/Engine.PrimitiveComponent))
  ;[1 1 1] Switch on or off?
  (if (Variables|Switch|GetSwitch%20Position%20On?)
    ;[1 1 1] Set switch and screen to glow when the switch is in the "on" position
    (bind _returnvalue_3 (Rendering|Material|GetVectorParameterValue _returnvalue "EmissiveMultiply" :!class /Script/Engine.MaterialInstanceDynamic))
    (Transformation|SetRelativeRotation _switch_button "300.000000,90.000000, 0" false false)
    (Rendering|Material|SetVectorParameterValueonMaterials _switch_button "EmissiveMultiply" (Math|Conversions|ToVector(LinearColor) _returnvalue_3))
    (bind _returnvalue_4 (Rendering|Material|GetVectorParameterValue _returnvalue_2 "EmissiveMultiply" :!class /Script/Engine.MaterialInstanceDynamic))
    (Rendering|Material|SetVectorParameterValueonMaterials _staticmeshcomponent "EmissiveMultiply" (Math|Conversions|ToVector(LinearColor) _returnvalue_4))
    (else
      ;[1 1 1] Set switch and screen to appeard off when the switch is in the "off" position
      (Transformation|SetRelativeRotation _switch_button "270.000000,90.000000, 0" false false)
      (Rendering|Material|SetVectorParameterValueonMaterials _switch_button "EmissiveMultiply" "0.000000,0.000000,0.000000")
      (Rendering|Material|SetVectorParameterValueonMaterials _staticmeshcomponent "EmissiveMultiply" "0, 0, 0"))))