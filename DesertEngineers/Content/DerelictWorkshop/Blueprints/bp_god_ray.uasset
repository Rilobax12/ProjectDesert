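; God ray actor that renders a configurable light shaft on a static mesh.
; The construction script creates a dynamic material, from an animated source when Animated is set, and optionally copies the rotation of an assigned Sun actor to the mesh's relative rotation.
; It then selects the mask texture by the SpotLight flag and pushes size, color, brightness, fade distance and a stream-seeded random value into material parameters.
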(fn ConstructionScript
  (bind _staticmesh1 (Variables|Default|GetStaticMesh1))
  (if (Variables|GodRay|GetAnimated)
    (bind _returnvalue (Rendering|Material|CreateDynamicMaterialInstance _staticmesh1 0 "/Game/DerelictWorkshop/Materials/Instances/mi_godray_a.mi_godray_a" :!class /Script/Engine.PrimitiveComponent)) ; Create and apply a dynamic material to the mesh that can be modified
    (Variables|GodRay|SetDynamic%20material _returnvalue)
    (else
      (bind _returnvalue_2 (Rendering|Material|CreateDynamicMaterialInstance _staticmesh1 0 0 :!class /Script/Engine.PrimitiveComponent))
      (Variables|GodRay|SetDynamic%20material _returnvalue_2)))
  (if (Variables|Default|GetUseSun) ; If true, the god ray will orient to match the rotation of the actor assigned to the "Sun" variable
    (Transformation|SetRelativeRotation (Variables|Default|GetStaticMesh1) (Transformation|GetActorRotation (Variables|GodRay|GetSun)) true false))
  (if (Variables|GodRay|GetSpotLight) ; If true, use a different falloff texture for the god ray material
    (Rendering|Material|SetTextureParameterValue (Variables|GodRay|GetDynamic%20material) "Mask" 0)
    (else
      (Rendering|Material|SetTextureParameterValue (Variables|GodRay|GetDynamic%20material) "Mask" "/Game/DerelictWorkshop/Textures/Lighting_Effects/t_god_ray_mask_a.t_god_ray_mask_a")))
  ;[1 1 1] Set various appearance parameters
  (Rendering|Material|SetScalarParameterValue (Variables|GodRay|GetDynamic%20material) "width" (Variables|GodRay|GetWidth) :!class /Script/Engine.MaterialInstanceDynamic)
  (Rendering|Material|SetScalarParameterValue (Variables|GodRay|GetDynamic%20material) "Length" (Variables|GodRay|GetLength) :!class /Script/Engine.MaterialInstanceDynamic)
  (Rendering|Material|SetVectorParameterValue (Variables|GodRay|GetDynamic%20material) "color" (Variables|GodRay|GetColor) :!class /Script/Engine.MaterialInstanceDynamic)
  (Rendering|Material|SetScalarParameterValue (Variables|GodRay|GetDynamic%20material) "Brightness" (Variables|GodRay|GetBrightness) :!class /Script/Engine.MaterialInstanceDynamic)
  (Rendering|Material|SetScalarParameterValue (Variables|GodRay|GetDynamic%20material) "fadedistance" (Variables|GodRay|GetFadeDistance) :!class /Script/Engine.MaterialInstanceDynamic)
  (Rendering|Material|SetScalarParameterValue (Variables|GodRay|GetDynamic%20material) "random" (Math|Random|RandomFloatinRangefromStream 0.0 1e+02 (Variables|GodRay|GetRandomTime)) :!class /Script/Engine.MaterialInstanceDynamic))